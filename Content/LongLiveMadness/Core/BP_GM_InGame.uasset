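; In-game GameMode that runs turn-based combat across rounds on a grid.
; Spawns player and colored-group characters from CharacterTurnStart markers due by the current round, sorting the turn queue by descending GAS Initiative.
; StartCombat restores units via abilities, initializes the HUD and starts the first turn.
; Each unit's GA_EndTurn callback advances turns, spawning newcomers as rounds wrap, with a resettable DoOnce guarding turn starts.
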(event `self.ReceiveBeginPlay`
  (`|ExecutionSequence`
    (:`then_0`
      (bind _returnvalue (`GameplayStatics.GetActorOfClass` "/Game/LongLiveMadness/World/GridSystem/BP_Grid.BP_Grid_C"))
      (set `self.GridActor` _returnvalue))
    (:`then_1`
      (`self.TrySpawnEnteringCharacters`))))

(event `StartCombat`
  (for (_array_element _array_index) (`self.TurnQueue`)
    (`AbilitySystemComponent.K2_GiveAbilityAndActivateOnce` (`MasterArbeitCharacter.AbilitySystemComponent` _array_element) "/Game/LongLiveMadness/TurnBasedSystem/GameplayAbility/GA_FullRestore.GA_FullRestore_C" 0 -1)
    (if (`|EnumEquality` (`MasterArbeitCharacter.CharacterGroupName` _array_element) "Player")
      (message `/Game/LongLiveMadness/Player/BPI_InGameHUD.SetPlayerTurnIndex` (`self.GetHUD`) _array_index)))
  (message `/Game/LongLiveMadness/Player/BPI_InGameHUD.InitAndLoadTurnOrderRelatedWidgets` (`self.GetHUD`) (`self.TurnQueue`))
  (`self.StartTurn`)
  (`self.NextTurn` (`self.ActiveTurn`)))

(event `StartTurn`
  (bind _output (`|GetArrayItem` (`self.TurnQueue`) (`self.ActiveTurn`)))
  (`/Engine/EditorBlueprintResources/StandardMacros.DoOnce` false :!label _label
    (:`Completed`
      (if (`KismetArrayLibrary.Array_IsValidIndex` (`self.TurnQueue`) (`self.ActiveTurn`))
        (`/Game/LongLiveMadness/Core/BP_BaseCharacter.StartUnitTurn` _output)
        (bind _asga_end_turn (cast `/Game/LongLiveMadness/TurnBasedSystem/GameplayAbility/GA_EndTurn` (`.ReturnValue` (`AbilitySystemBlueprintLibrary.GetGameplayAbilityFromSpecHandle` (`AbilitySystemBlueprintLibrary.GetAbilitySystemComponent` _output) (`/Game/LongLiveMadness/Core/BP_BaseCharacter.EndTurn_SH` _output))))
          (:`then`
            (add `/Game/LongLiveMadness/TurnBasedSystem/GameplayAbility/GA_EndTurn.EndTurn` _asga_end_turn (delegate `OnTurnEnd`)))
          (:`CastFailed`
            (`KismetSystemLibrary.PrintString` "Not End Turn Ability")))
        (else
          (`self.ReadyNextTurn`))))))

(event `ReadyNextTurn`
  (`|ExecutionSequence`
    (:`then_0`
      (goto _label :!via `Reset`))
    (:`then_1`
      (if (`KismetArrayLibrary.Array_IsValidIndex` (`self.TurnQueue`) (`self.ActiveTurn`))
        (`self.StartTurn`)))))

(event `OnTurnEnd`
  (params (EndTurnAbility :type "/Game/LongLiveMadness/TurnBasedSystem/GameplayAbility/GA_EndTurn Object Reference"))
  (clear `/Game/LongLiveMadness/TurnBasedSystem/GameplayAbility/GA_EndTurn.EndTurn` EndTurnAbility)
  (if (>= (`self.ActiveTurn`) (- (`KismetArrayLibrary.Array_Length` (`self.TurnQueue`)) 1))
    (set `self.ActiveTurn` 0)
    (bind _result (`/Engine/EditorBlueprintResources/StandardMacros.IncrementInt` (`self.ActiveRound`))
      (:`  `
        (bind _newspawned (`self.TrySpawnEnteringCharacters`))
        (if (> (`KismetArrayLibrary.Array_Length` _newspawned) 0)
          ;[0.04394 0.8438 0.3266 0.5] -> to function or macro
          (for _array_element _newspawned
            (`AbilitySystemComponent.K2_GiveAbilityAndActivateOnce` (`MasterArbeitCharacter.AbilitySystemComponent` _array_element) "/Game/LongLiveMadness/TurnBasedSystem/GameplayAbility/GA_FullRestore.GA_FullRestore_C" 0 -1))
          (message `/Game/LongLiveMadness/Player/BPI_InGameHUD.RefreshTurnOrderRelatedWidgets` (`self.GetHUD`) (`self.TurnQueue`)))
        (`self.NextRound` _result)))
    (else
      (`/Engine/EditorBlueprintResources/StandardMacros.IncrementInt` (`self.ActiveTurn`)
        (:`  `
          _))))
  (`self.NextTurn` (`self.ActiveTurn`))
  (`self.ReadyNextTurn`))

(fn `CharacterInitiativeComparator`
  (params (`Object A` :type "Object Object Reference") (`Object B` :type "Object Object Reference"))
  (returns (Boolean :type Boolean))
  (bind _asbp_base_character (cast `/Game/LongLiveMadness/Core/BP_BaseCharacter` `Object A`))
  (bind _returnvalue (`AbilitySystemComponent.GetAttributeSet` (`MasterArbeitCharacter.AbilitySystemComponent` _asbp_base_character) "/Script/TurnBasedCombatSystem.CombatAttributeSet"))
  (bind _asbp_base_character_2 (cast `/Game/LongLiveMadness/Core/BP_BaseCharacter` `Object B`))
  (bind _returnvalue_2 (`AbilitySystemComponent.GetAttributeSet` (`MasterArbeitCharacter.AbilitySystemComponent` _asbp_base_character_2) "/Script/TurnBasedCombatSystem.CombatAttributeSet"))
  (return (< (`.BaseValue` (break `GameplayAttributeData` (`CombatAttributeSet.Initiative` _returnvalue))) (`.BaseValue` (break `GameplayAttributeData` (`CombatAttributeSet.Initiative` _returnvalue_2))))))

(fn `GetGridActor`
  (returns (GridActor :type "/Game/LongLiveMadness/World/GridSystem/BP_Grid Object Reference"))
  (return (`self.GridActor`)))

(fn `RefreshTurnOrder`
  (params (CurrentTurnOrder :type "Array of /Game/LongLiveMadness/Core/BP_BaseCharacter Object Reference"))
  (returns (RefreshedTurnOrder :type "Array of /Game/LongLiveMadness/Core/BP_BaseCharacter Object Reference"))
  (`LowEntryExtendedStandardLibrary.SortObjectArrayDirectly` CurrentTurnOrder (`|CreateDelegate` :!event `CharacterInitiativeComparator`) true)
  (return))

(fn `SpawnCharacterAtStartPosition`
  (params (Start :type "CharacterTurnStart Object Reference"))
  (returns (Spawned :type "/Game/LongLiveMadness/Core/BP_BaseCharacter Object Reference"))
  (bind _charactergroupname (`CharacterTurnStart.CharacterGroupName` Start))
  (bind _returnvalue (`|SpawnActorFromClass` (select `ECharacterGroupName` _charactergroupname :`Player` "/Game/LongLiveMadness/Player/BP_PlayerCharacter.BP_PlayerCharacter_C" :`Green` "/Game/LongLiveMadness/LlamaAgent/Character/BP_Green.BP_Green_C" :`Red` "/Game/LongLiveMadness/LlamaAgent/Character/BP_Red.BP_Red_C" :`Purple` "/Game/LongLiveMadness/LlamaAgent/Character/BP_Purple.BP_Purple_C" :!type "Actor Class Reference") (`self.GetTransform` (`local.Start`)) "AdjustIfPossibleButAlwaysSpawn" "MultiplyWithRoot" null (`self.GetInstigator`)))
  (bind _asbp_base_character (cast `/Game/LongLiveMadness/Core/BP_BaseCharacter` _returnvalue)
    (:`then`
      (if (`|EnumEquality` _charactergroupname "Player")
        (`Controller.Possess` (`GameplayStatics.GetPlayerController` 0) _asbp_base_character))
      (`KismetArrayLibrary.Array_AddUnique` (`self.TurnQueue`) _asbp_base_character)
      (`self.K2_DestroyActor` (`local.Start`))
      (return _asbp_base_character))
    (:`CastFailed`
      (return null))))

(fn `TrySpawnEnteringCharacters`
  (returns (NewSpawned :type "Array of /Game/LongLiveMadness/Core/BP_BaseCharacter Object Reference"))
  (locals (NewSpawnedCharacters :type "Array of /Game/LongLiveMadness/Core/BP_BaseCharacter Object Reference"))
  (bind _outactors (`GameplayStatics.GetAllActorsOfClass` "/Script/MasterArbeit.CharacterTurnStart"))
  (for _array_element _outactors
    (if (<= (`CharacterTurnStart.StartTurnIndex` _array_element) (`self.ActiveRound`))
      (bind _spawned (`self.SpawnCharacterAtStartPosition` _array_element))
      (`KismetArrayLibrary.Array_AddUnique` (`local.NewSpawnedCharacters`) _spawned)))
  (`LowEntryExtendedStandardLibrary.SortObjectArrayDirectly` (`self.TurnQueue`) (`|CreateDelegate` :!event `CharacterInitiativeComparator`) true)
  (return (`local.NewSpawnedCharacters`)))

(fn `UserConstructionScript`)