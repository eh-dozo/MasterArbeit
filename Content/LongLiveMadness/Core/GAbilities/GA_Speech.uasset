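; GA_Speech is an event-triggered gameplay ability through which a character speaks a chat message.
; It responds only to events whose optional object is a CharacterChatMessageWrapper.
; On activation it broadcasts that message through the TextCommunicationSubsystem, records the text as a verbal interaction on the owning BP_BaseCharacter's TurnActionTracker, then ends.
; The ability cost commit is left unconnected, so speech commits no cost.
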(event `self.K2_ActivateAbilityFromEvent`
  (params (EventData :type "GameplayEventData Structure (by ref)"))
  (bind _ascharacter_chat_message_wrapper (cast `CharacterChatMessageWrapper` (`.OptionalObject` (break `GameplayEventData` EventData)))
    (:`then`
      (bind _characterchatmessage (`CharacterChatMessageWrapper.CharacterChatMessage` _ascharacter_chat_message_wrapper))
      (`TextCommunicationSubsystem.AddCharacterChatMessage` (subsystem `TextCommunicationSubsystem`) _characterchatmessage true)
      (bind _asbp_base_character (cast `/Game/LongLiveMadness/Core/BP_BaseCharacter` (`self.GetOwningActorFromActorInfo`)))
      (`TurnActionTrackerComponent.RecordVerbalInteraction` (`/Game/LongLiveMadness/Core/BP_BaseCharacter.TurnActionTracker` _asbp_base_character) (`KismetTextLibrary.Conv_TextToString` (`.Message` (break `CharacterChatMessage` _characterchatmessage))))
      (`self.K2_EndAbility`))
    (:`CastFailed`
      (`KismetSystemLibrary.PrintString` "Can't cast chat message wrapper" true true (struct :`G` 0.66 :`B` 1.0 :`A` 1.0) 5.0))))

(fn `K2_ShouldAbilityRespondToEvent`
  (params (ActorInfo :type "GameplayAbilityActorInfo Structure") (Payload :type "GameplayEventData Structure"))
  (returns (ReturnValue :type Boolean))
  (cast `CharacterChatMessageWrapper` (`.OptionalObject` (break `GameplayEventData` Payload))
    (:`then`
      (return true))
    (:`CastFailed`
      (return false))))