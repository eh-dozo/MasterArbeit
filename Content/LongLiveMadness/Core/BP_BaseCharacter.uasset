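; Base character for turn-based combat units, built on the Gameplay Ability System and tinted by character group.
; Construction gets a theme color from the group name and applies it to two dynamic mesh materials.
; BeginPlay binds the CombatAttributeSet to the world health bar widget.
; Turn start grants damage-self, end-turn and speech abilities, then signals turn start; turn end activates the end-turn ability and clears all abilities.
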(event `self.ReceiveBeginPlay`
  (bind _asbpw_health_bar_world (cast `/Game/LongLiveMadness/UI/InGame/HealthBar/BPW_HealthBarWorld` (`WidgetComponent.GetUserWidgetObject` (`self.Widget_HealthBar`))))
  (bind _returnvalue (`AbilitySystemComponent.GetAttributeSet` (`self.AbilitySystemComponent`) "/Script/TurnBasedCombatSystem.CombatAttributeSet"))
  (`/Engine/EditorBlueprintResources/StandardMacros.IsValid` _returnvalue
    (:`Is Valid`
      (`/Game/LongLiveMadness/UI/InGame/HealthBar/BPW_HealthBarWorld.SetCombatAttributeSet` _asbpw_health_bar_world _returnvalue))
    (:`Is Not Valid`
      (`KismetSystemLibrary.PrintText` (`|FormatText` "Couldn't get combat attribute set for {0}" (`KismetSystemLibrary.GetDisplayName` self))))))

(event `StartUnitTurn`
  (bind _returnvalue (`AbilitySystemComponent.K2_GiveAbility` (`self.AbilitySystemComponent`) "/Game/LongLiveMadness/TurnBasedSystem/GameplayAbility/GA_DamageSelf.GA_DamageSelf_C" 0 -1))
  (set `self.DamageSelf_SH` _returnvalue)
  (bind _returnvalue_2 (`AbilitySystemComponent.K2_GiveAbility` (`self.AbilitySystemComponent`) "/Game/LongLiveMadness/TurnBasedSystem/GameplayAbility/GA_EndTurn.GA_EndTurn_C" 0 -1))
  (set `self.EndTurn_SH` _returnvalue_2)
  (bind _returnvalue_3 (`AbilitySystemComponent.K2_GiveAbility` (`self.AbilitySystemComponent`) "/Game/LongLiveMadness/TurnBasedSystem/GameplayAbility/GA_Speech.GA_Speech_C" 0 -1))
  (set `self.Speech_SH` _returnvalue_3)
  (`self.OnTurnStart`))

(event `EndUnitTurn`
  (`AbilitySystemComponent.TryActivateAbility` (`self.AbilitySystemComponent`) (`self.EndTurn_SH`) true)
  (`AbilitySystemComponent.ClearAllAbilities` (`self.AbilitySystemComponent`)))

(fn `UserConstructionScript`
  (bind _themecolor (`/Game/LongLiveMadness/Core/Extra/BPL_CharacterThemes.GetCharacterThemeColor` (`self.CharacterGroupName`)))
  (set `self.ThemeColor` _themecolor)
  (bind _returnvalue (`PrimitiveComponent.CreateDynamicMaterialInstance` (`self.Mesh`) 0 "/Game/Characters/Mannequins/Materials/Instances/Quinn/MI_Quinn_01.MI_Quinn_01" "None"))
  (`MaterialInstanceDynamic.SetVectorParameterValue` _returnvalue "Tint" (`self.ThemeColor`))
  (bind _returnvalue_2 (`PrimitiveComponent.CreateDynamicMaterialInstance` (`self.Mesh`) 1 "/Game/Characters/Mannequins/Materials/Instances/Quinn/MI_Quinn_02.MI_Quinn_02" "None"))
  (`MaterialInstanceDynamic.SetVectorParameterValue` _returnvalue_2 "Tint" (`self.ThemeColor`)))