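; Player movement Gameplay Ability, triggered by an event whose payload wrapper carries the target location, and blocked while already active.
; It charges movement points through a cached SetByCaller cost effect scaled by straight-line distance to the target.
; Once the cost commits, an async task waits for the move to complete, then logs it in the character's TurnActionTracker.
; Failures print a message and cancel or end the ability; the cursor FX spawn is unconnected.
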(event `self.K2_ActivateAbilityFromEvent`
  (params (EventData :type "GameplayEventData Structure (by ref)"))
  (bind _asplayer_ability_movement_payload_wrapper (cast `PlayerAbilityMovementPayloadWrapper` EventData_OptionalObject)
    (:`then`
      (bind _playerabilitymovementpayload_targetlocation (break `PlayerAbilityMovementPayload` (`PlayerAbilityMovementPayloadWrapper.PlayerAbilityMovementPayload` _asplayer_ability_movement_payload_wrapper)))
      (bind _output_get (set `self.TargetLocation` _playerabilitymovementpayload_targetlocation))
      (bind _returnvalue (`AbilitySystemBlueprintLibrary.AssignTagSetByCallerMagnitude` (`self.MakeOutgoingGameplayEffectSpec` "/Game/LongLiveMadness/Player/GEffects/GE_Cost_MovementPoints_Player.GE_Cost_MovementPoints_Player_C") (struct :`TagName` "Abilities.Data.TurnCost") (/ (`KismetMathLibrary.Vector_Distance` _output_get (`Actor.K2_GetActorLocation` (`self.GetOwningActorFromActorInfo`))) -250.0)))
      (`self.SetCachedCostEffectSpec` _returnvalue)
      (bind _returnvalue_2 (`self.K2_CommitAbilityCost` false))
      (if _returnvalue_2
        (bind _asbp_player_character (cast `/Game/LongLiveMadness/Player/BP_PlayerCharacter` (`self.GetOwningActorFromActorInfo`))
          (:`then`
            (`GATSimpleCharacterMoveTo.WaitForCharacterMovementToComplete` (`self.TargetLocation`)
              (:`OnMovementComplete`
                (`TurnActionTrackerComponent.RecordMovement` (`/Game/LongLiveMadness/Core/BP_BaseCharacter.TurnActionTracker` _asbp_player_character) "continued to move forward along the road")
                (`self.K2_EndAbility`))
              (:`OnMovementFailed`
                (`KismetSystemLibrary.PrintString` "Cancel Player Move: fail AI move to" true true (struct :`R` 1.0 :`G` 0.059236 :`A` 1.0) 20.0)
                (`self.K2_CancelAbility` :!label _label))))
          (:`CastFailed`
            (`KismetSystemLibrary.PrintString` "Cancel Player Move: can't cast player character" true true (struct :`R` 1.0 :`G` 0.059236 :`A` 1.0) 20.0)
            (goto _label)))
        (else
          (`KismetSystemLibrary.PrintString` "Cancel Player Move: can't commit cost" true true (struct :`R` 1.0 :`G` 0.059236 :`A` 1.0) 20.0)
          (`self.K2_EndAbility`))))
    (:`CastFailed`
      (`KismetSystemLibrary.PrintString` "Cancel Player Move: can't cast wrapper" true true (struct :`R` 1.0 :`G` 0.059236 :`A` 1.0) 20.0)
      (goto _label))))

(fn `K2_CanActivateAbility`
  (params (ActorInfo :type "GameplayAbilityActorInfo Structure") (Handle :type "GameplayAbilitySpecHandle Structure"))
  (returns (RelevantTags :type "GameplayTagContainer Structure") (ReturnValue :type Boolean))
  (return (struct) (not (`AbilitySystemBlueprintLibrary.IsGameplayAbilityActive` null))))

(fn `K2_ShouldAbilityRespondToEvent`
  (params (ActorInfo :type "GameplayAbilityActorInfo Structure") (Payload :type "GameplayEventData Structure"))
  (returns (ReturnValue :type Boolean))
  (cast `PlayerAbilityMovementPayloadWrapper` Payload_OptionalObject
    (:`then`
      (return true))
    (:`CastFailed`
      (return false))))