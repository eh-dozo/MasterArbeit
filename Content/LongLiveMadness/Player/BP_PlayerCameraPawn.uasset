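; Player camera pawn that moves over the landscape, rotates in 90-degree steps and zooms.
; A curve-driven zoom value blends arm length, pitch, FOV and move speed, with depth of field following arm length.
; Movement starts looping timers that trace ground height and update an occlusion point offset toward the camera.
; Tick smoothly snaps pawn height and feeds that point into a Material Parameter Collection for fading occluders.
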(event `self.ReceiveBeginPlay`
  (`self.UpdateZoom` 0.0)
  (bind _adjustedoccludedposition (`self.SetGroundOccludePosition`))
  (`KismetMaterialLibrary.SetVectorParameterValue` "/Game/LongLiveMadness/Art/Common/OcclusionCutout/MPC_Camera_Occlusion.MPC_Camera_Occlusion" "CameraAvatarPosition" (`KismetMathLibrary.Conv_VectorToLinearColor` _adjustedoccludedposition))
  (bind (_adjustedlandscapeheight _ishit) (`self.GetLandscapeHeightUnderActor`))
  (if _ishit
    (set `self.AdjustedLandscapeHeight` _adjustedlandscapeheight)))

(event `self.ReceiveTick`
  (params (DeltaSeconds :type "Float (single-precision)"))
  (bind _returnvalue (`self.K2_GetActorLocation`))
  (`|ExecutionSequence`
    (:`then_0`
      (`self.K2_SetActorLocation` (`KismetMathLibrary.VInterpTo` _returnvalue (`KismetMathLibrary.MakeVector` (.x _returnvalue) (.y _returnvalue) (`self.AdjustedLandscapeHeight`)) (`GameplayStatics.GetWorldDeltaSeconds`) (`self.SnappingInterSpeed`))))
    (:`then_1`
      (bind _returnvalue_2 (`KismetMaterialLibrary.GetVectorParameterValue` "/Game/LongLiveMadness/Art/Common/OcclusionCutout/MPC_Camera_Occlusion.MPC_Camera_Occlusion" "CameraAvatarPosition"))
      (`KismetMaterialLibrary.SetVectorParameterValue` "/Game/LongLiveMadness/Art/Common/OcclusionCutout/MPC_Camera_Occlusion.MPC_Camera_Occlusion" "CameraAvatarPosition" (`KismetMathLibrary.Conv_VectorToLinearColor` (`KismetMathLibrary.VInterpTo` (`KismetMathLibrary.MakeVector` (break `LinearColor` _returnvalue_2) (`.G` (break `LinearColor` _returnvalue_2)) (`.B` (break `LinearColor` _returnvalue_2))) (`self.OccludePosition`) (`GameplayStatics.GetWorldDeltaSeconds`) 11.0))))))

(event `TraceLandscapeHeight`
  ;[0.1119 0.6445 0.4397 0.502] Track highest landscape height under the pawn
  (if (`self.IsStopped`)
    (`KismetSystemLibrary.K2_ClearAndInvalidateTimerHandle` (`self.TrackLandscapeHeightTimer`))
    (goto _label :!via `Reset`)
    (else
      (bind (_adjustedlandscapeheight _ishit) (`self.GetLandscapeHeightUnderActor`))
      (if _ishit
        (set `self.AdjustedLandscapeHeight` _adjustedlandscapeheight)))))

(event `OnPawnStateChange_Move`
  (`|ExecutionSequence`
    (:`then_0`
      ;[0.1119 0.6445 0.4397 0.502] Track highest landscape height under the pawn
      (`/Engine/EditorBlueprintResources/StandardMacros.DoOnce` false :!label _label
        (:`Completed`
          (bind _returnvalue (`KismetSystemLibrary.K2_SetTimerDelegate` (delegate `TraceLandscapeHeight`) 0.1 true true))
          (set `self.TrackLandscapeHeightTimer` _returnvalue))))
    (:`then_1`
      ;[0.1119 0.6445 0.4397 0.502] Track on-ground camera position and camera occlusion
      (`/Engine/EditorBlueprintResources/StandardMacros.DoOnce` false :!label _label_2
        (:`Completed`
          (bind _returnvalue_2 (`KismetSystemLibrary.K2_SetTimerDelegate` (delegate `TracePosition`) 0.1 true true))
          (set `self.TrackPositionTimer` _returnvalue_2))))))

(event `TracePosition`
  ;[0.1119 0.6445 0.4397 0.502] Track on-ground camera position and camera occlusion
  (if (`self.IsStopped`)
    (`KismetSystemLibrary.K2_ClearAndInvalidateTimerHandle` (`self.TrackPositionTimer`))
    (goto _label_2 :!via `Reset`)
    (else
      (`self.SetGroundOccludePosition`))))

(fn `Dof`
  (set `CameraComponent.PostProcessSettings` (make `PostProcessSettings` :`DepthOfFieldFstop` 3.0 :`DepthOfFieldSensorWidth` 150.0 :`DepthOfFieldFocalDistance` (+ (`SpringArmComponent.TargetArmLength` (`self.SpringArm`)) 350.0)) (`self.Camera`)))

(fn `MoveCamera`
  (params (Direction :type "Vector2D Structure"))
  (bind (_x _y) (`KismetMathLibrary.BreakVector2D` Direction))
  (`self.AddMovementInput` (`self.GetActorRightVector`) (* _x (`self.MovementSpeed`)))
  (`self.AddMovementInput` (`self.GetActorForwardVector`) (* _y (`self.MovementSpeed`)))
  (`self.OnPawnStateChange_Move`))

(fn `RotateCamera`
  (params (Direction :type Boolean))
  (if Direction
    (`self.K2_AddActorLocalRotation` (struct :`Yaw` 90.0))
    (else
      (`self.K2_AddActorLocalRotation` (struct :`Yaw` -90.0)))))

(fn `SnapCursorToLandscape`
  (`self.K2_SetActorLocation` (`KismetMathLibrary.VInterpTo` (`self.K2_GetActorLocation`) (+ (`self.AdjustedLandscapeHeight`) (`KismetMathLibrary.MakeVector` 0.0 0.0 (`self.CursorSnappingOffset`))) (`GameplayStatics.GetWorldDeltaSeconds`) (`self.SnappingInterSpeed`))))

(fn `UpdateZoom`
  (params (ZoomDirection :type "Float (double-precision)"))
  (bind _springarm (`self.SpringArm`))
  (bind _returnvalue (`CurveFloat.GetFloatValue` (`self.ZoomCurve`) (`self.ZoomValue`)))
  (set `self.ZoomDirection` ZoomDirection)
  (set `self.ZoomValue` (`KismetMathLibrary.FClamp` (+ (* (`self.ZoomDirection`) (`self.ZoomStrenght`)) (`self.ZoomValue`))))
  (set `SpringArmComponent.TargetArmLength` (`KismetMathLibrary.Lerp` 5000.0 15000.0 _returnvalue) _springarm)
  (`SceneComponent.K2_SetRelativeRotation` _springarm (`KismetMathLibrary.MakeRotator` 0.0 (`KismetMathLibrary.Lerp` -30.0 -55.0 _returnvalue)) false false)
  (set `FloatingPawnMovement.MaxSpeed` (`KismetMathLibrary.Lerp` 1000.0 6000.0 _returnvalue) (`self.FloatingPawnMovement`))
  (`self.Dof`)
  (`CameraComponent.SetFieldOfView` (`self.Camera`) (`KismetMathLibrary.Lerp` 20.0 15.0 _returnvalue)))

(fn `UserConstructionScript`)