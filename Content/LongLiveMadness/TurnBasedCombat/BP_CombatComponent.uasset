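; Actor component that represents a combat unit in the turn-based combat system.
; On BeginPlay it casts its owner to TBCControllerInterface, caches it, and records the owning actor's transform as the battle position.
; EndUnitTurn fires the TurnEnd dispatcher with itself as the argument.
; StartUnitTurn and BeginCombat are empty stubs, and a delayed turn-end chain is left disconnected.
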(event `self.ReceiveBeginPlay`
  (bind _astbccontroller_interface (cast `TBCControllerInterface` (`self.GetOwner`)))
  (bind _output_get (set `self.TBCController` _astbccontroller_interface))
  (bind _returnvalue (`TBCControllerInterface.GetOwningActorTransform` _output_get))
  (set `self.BattlePosition` _returnvalue))

(event `self.StartUnitTurn`)

(event `self.EndUnitTurn`
  (`self.TurnEnd` self))

(event `self.BeginCombat`)