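; Player camera pawn with an orthographic camera on a spring arm, offering move, zoom and 90-degree yaw rotation functions.
; Each tick a downward line trace eases the pawn toward a set offset above the surface below it.
; A clamped zoom value, shaped by a curve, drives spring arm pitch, ortho width and movement max speed together, so wider views pan faster.
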(event `self.ReceiveBeginPlay`
  (`self.UpdateZoom` 0.0))

(event `self.ReceiveTick`
  (params (DeltaSeconds :type "Float (single-precision)"))
  (`self.SnapCursorToLandscape`))

(fn `MoveCamera`
  (params (Direction :type "Vector2D Structure"))
  (bind (_x _y) (`KismetMathLibrary.BreakVector2D` Direction))
  (`self.AddMovementInput` (`self.GetActorRightVector`) (* _x (`self.MovementSpeed`)))
  (`self.AddMovementInput` (`self.GetActorForwardVector`) (* _y (`self.MovementSpeed`))))

(fn `RotateCamera`
  (params (Direction :type Boolean))
  (if Direction
    (`self.K2_AddActorLocalRotation` (struct :`Yaw` 90.0))
    (else
      (`self.K2_AddActorLocalRotation` (struct :`Yaw` -90.0)))))

(fn `SnapCursorToLandscape`
  (bind _returnvalue (`self.K2_GetActorLocation`))
  (bind (_outhit _returnvalue_2) (`KismetSystemLibrary.LineTraceSingle` _returnvalue (`KismetMathLibrary.MakeVector` (.x _returnvalue) (.y _returnvalue) (- (.z _returnvalue) 1000.0)) "TraceTypeQuery3"))
  (if _returnvalue_2
    (`self.K2_SetActorLocation` (`KismetMathLibrary.VInterpTo` (`self.K2_GetActorLocation`) (+ (`.Location` (`GameplayStatics.BreakHitResult` _outhit)) (`KismetMathLibrary.MakeVector` 0.0 0.0 (`self.CursorSnappingOffset`))) (`GameplayStatics.GetWorldDeltaSeconds`) (`self.SnappingInterSpeed`)))))

(fn `UpdateZoom`
  (params (ZoomDirection :type "Float (double-precision)"))
  (bind _returnvalue (`CurveFloat.GetFloatValue` (`self.ZoomCurve`) (`self.ZoomValue`)))
  (set `self.ZoomDirection` ZoomDirection)
  (set `self.ZoomValue` (`KismetMathLibrary.FClamp` (+ (* (`self.ZoomDirection`) (`self.ZoomStrenght`)) (`self.ZoomValue`))))
  (`SceneComponent.K2_SetRelativeRotation` (`self.SpringArm`) (`KismetMathLibrary.MakeRotator` 0.0 (`KismetMathLibrary.Lerp` -30.0 -55.0 _returnvalue)) false false)
  (set `FloatingPawnMovement.MaxSpeed` (`KismetMathLibrary.Lerp` 1000.0 6000.0 _returnvalue) (`self.FloatingPawnMovement`))
  (`CameraComponent.SetOrthoWidth` (`self.Camera`) (`KismetMathLibrary.Lerp` 850.0 5000.0 _returnvalue)))

(fn `UserConstructionScript`)