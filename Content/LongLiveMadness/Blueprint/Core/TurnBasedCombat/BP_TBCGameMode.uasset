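; Game mode for turn-based combat that runs controllers' turns one at a time from a queue.
; RequestTurn adds a unique controller to TurnQueue and tries to start it through a DoOnce gate.
; StartTurn starts the first controller's combat component, binds its turn-end event and dequeues it.
; Turn end resets the gate and starts the next queued turn; BeginPlay only prints the player state count.
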(event `self.ReceiveBeginPlay`
  (`KismetSystemLibrary.PrintString` (`KismetStringLibrary.Conv_IntToString` (`GameplayStatics.GetNumPlayerStates`))))

(event `RequestTurn`
  (params (TBCController :type "TBCControllerInterface Interface"))
  (`KismetArrayLibrary.Array_AddUnique` (`self.TurnQueue`) TBCController)
  (`self.StartTurn`))

(event `StartTurn`
  (`/Engine/EditorBlueprintResources/StandardMacros.DoOnce` false :!label _label
    (:`Completed`
      (if (`KismetArrayLibrary.Array_IsValidIndex` (`self.TurnQueue`))
        (bind _returnvalue (`TBCControllerInterface.GetCombatComponent` (`|GetArrayItem` (`self.TurnQueue`))))
        (`CombatComponent.StartUnitTurn` _returnvalue)
        (add `CombatComponent.OnTurnEnd` _returnvalue (delegate `OnTurnEnd_Event`))
        (`KismetArrayLibrary.Array_Remove` (`self.TurnQueue`))
        (else
          (`self.ReadyNextTurn`))))))

(event `ReadyNextTurn`
  (`|ExecutionSequence`
    (:`then_0`
      (goto _label :!via `Reset`))
    (:`then_1`
      (if (`KismetArrayLibrary.Array_IsValidIndex` (`self.TurnQueue`))
        (`self.StartTurn`)))))

(event `OnTurnEnd_Event`
  (`self.ReadyNextTurn`))

(fn `UserConstructionScript`)