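; Combat grid actor that maps world positions to tiles and supplies tile locations for placing human-sized characters.
; It pushes size, color, line and offset settings into the MPC_CombatGrid parameter collection on construction and BeginPlay.
; Parent-function overrides snap positions to tile centers or resolve row/column to ground points via downward traces with a half-height lift.
; A random-tile function returns a similarly traced transform with a random diagonal yaw.
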(event `self.ReceiveBeginPlay`
  (`self.InitGridMaterialParameters`))

(fn `GetRandomTileLocation`
  (returns (RandomTile :type "Transform Structure"))
  (bind (_x _y) (`self.ComputeTileCenter` (`KismetMathLibrary.RandomInteger` (`self.Rows`)) (`KismetMathLibrary.RandomInteger` (`self.Columns`))))
  (bind (_outhit _returnvalue) (`KismetSystemLibrary.LineTraceSingle` (`KismetMathLibrary.MakeVector` _x _y 3000.0) (`KismetMathLibrary.MakeVector` _x _y 1000.0) "TraceTypeQuery3"))
  (if _returnvalue
    (return (`KismetMathLibrary.MakeTransform` (`KismetMathLibrary.MakeVector` (.x (`.Location` (`GameplayStatics.BreakHitResult` _outhit))) (.y (`.Location` (`GameplayStatics.BreakHitResult` _outhit))) (+ (.z (`.Location` (`GameplayStatics.BreakHitResult` _outhit))) (`self.HumanSizeHalfSizeOffset`))) (`KismetMathLibrary.MakeRotator` 0.0 0.0 (+ 45.0 (* 90 (`KismetMathLibrary.RandomInteger` 3))))))))

(fn `GetTileLocation`
  (params (Row :type Integer) (Col :type Integer))
  (returns (OutTileLocation :type "Vector Structure") (ReturnValue :type Boolean))
  (bind (_x _y) (`self.ComputeTileCenter` (`local.Row`) (`local.Col`)))
  (`parent.GetTileLocation` Row Col)
  (if (`self.AreCoordinatesInGrid` (`local.Row`) (`local.Col`))
    (bind (_outhit _returnvalue) (`KismetSystemLibrary.LineTraceSingle` (`KismetMathLibrary.MakeVector` _x _y 3000.0) (`KismetMathLibrary.MakeVector` _x _y 1000.0) "TraceTypeQuery3"))
    (if _returnvalue
      (return (`KismetMathLibrary.MakeVector` (.x (`.Location` (`GameplayStatics.BreakHitResult` _outhit))) (.y (`.Location` (`GameplayStatics.BreakHitResult` _outhit))) (+ (.z (`.Location` (`GameplayStatics.BreakHitResult` _outhit))) (`self.HumanSizeHalfSizeOffset`))) true)
      (else
        (return (0.0 0.0 0.0) false)))
    (else
      (return (0.0 0.0 0.0) false))))

(fn `InitGridMaterialParameters`
  (`KismetMaterialLibrary.SetVectorParameterValue` "/Game/LongLiveMadness/Blueprint/World/GridSystem/Material/MPC_CombatGrid.MPC_CombatGrid" "Ground color" (`self.Ground Color`))
  (`KismetMaterialLibrary.SetVectorParameterValue` "/Game/LongLiveMadness/Blueprint/World/GridSystem/Material/MPC_CombatGrid.MPC_CombatGrid" "Line tint" (`self.Line Tint`))
  (`KismetMaterialLibrary.SetScalarParameterValue` "/Game/LongLiveMadness/Blueprint/World/GridSystem/Material/MPC_CombatGrid.MPC_CombatGrid" "Tile size" (`self.Tile Size`))
  (`KismetMaterialLibrary.SetScalarParameterValue` "/Game/LongLiveMadness/Blueprint/World/GridSystem/Material/MPC_CombatGrid.MPC_CombatGrid" "Line width" (`self.Line width`))
  (`KismetMaterialLibrary.SetScalarParameterValue` "/Game/LongLiveMadness/Blueprint/World/GridSystem/Material/MPC_CombatGrid.MPC_CombatGrid" "Rows" (`KismetMathLibrary.Conv_IntToDouble` (`self.Rows`)))
  (`KismetMaterialLibrary.SetScalarParameterValue` "/Game/LongLiveMadness/Blueprint/World/GridSystem/Material/MPC_CombatGrid.MPC_CombatGrid" "Columns" (`KismetMathLibrary.Conv_IntToDouble` (`self.Columns`)))
  (`KismetMaterialLibrary.SetVectorParameterValue` "/Game/LongLiveMadness/Blueprint/World/GridSystem/Material/MPC_CombatGrid.MPC_CombatGrid" "Offset" (`self.Offset`)))

(fn `LocateTileCenter`
  (params (CachedDestination :type "Vector Structure (by ref)"))
  (returns (OutTileCenter :type "Vector Structure") (ReturnValue :type Boolean))
  (locals (RowLocation :type Integer :default 0) (ColumnLocation :type Integer :default 0))
  (bind (_row _column) (`self.ConvertLocationToGridCoordinates` (`local.CachedDestination`)))
  (bind (_x _y) (`self.ComputeTileCenter` (`local.RowLocation`) (`local.ColumnLocation`)))
  (`parent.LocateTileCenter` CachedDestination)
  (if (and (> (`self.Rows`) 0) (> (`self.Columns`) 0))
    (set `local.RowLocation` _row)
    (set `local.ColumnLocation` _column)
    (if (`self.AreCoordinatesInGrid` (`local.RowLocation`) (`local.ColumnLocation`))
      (return (`KismetMathLibrary.MakeVector` _x _y (.z (`local.CachedDestination`))) true)
      (else
        (`KismetSystemLibrary.PrintString` "Not inside")
        (return (0.0 0.0 0.0) false)))
    (else
      (return (0.0 0.0 0.0) false))))

(fn `UserConstructionScript`
  (`self.InitGridMaterialParameters`))