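; GA_FullHeal is a Gameplay Ability for the turn-based combat system that restores its owner to full health.
; On activation it reads the CombatAttributeSet and computes the missing health as MaxHealth minus current Health.
; It passes that amount as a SetByCaller magnitude to a GE_Heal spec, applies it to its own ability system component, and ends immediately.
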(event `self.K2_ActivateAbility`
  (bind _returnvalue (`AbilitySystemComponent.GetAttributeSet` (`self.GetAbilitySystemComponentFromActorInfo`) "/Script/TurnBasedCombatSystem.CombatAttributeSet"))
  (bind _returnvalue_2 (`AbilitySystemBlueprintLibrary.MakeSpecHandleByClass` "/Game/LongLiveMadness/TurnBasedSystem/GameplayEffect/GE_Heal.GE_Heal_C"))
  (bind _returnvalue_3 (`AbilitySystemBlueprintLibrary.AssignTagSetByCallerMagnitude` _returnvalue_2 (struct :`TagName` "Abilities.Parameters.Heal") (- (`.CurrentValue` (break `GameplayAttributeData` (`CombatAttributeSet.MaxHealth` _returnvalue))) (`.CurrentValue` (break `GameplayAttributeData` (`CombatAttributeSet.Health` _returnvalue))))))
  (`AbilitySystemComponent.BP_ApplyGameplayEffectSpecToSelf` (`self.GetAbilitySystemComponentFromActorInfo`) _returnvalue_3)
  (`self.K2_EndAbility`))