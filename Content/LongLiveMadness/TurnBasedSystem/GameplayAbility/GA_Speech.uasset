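; GA_Speech is a turn-based gameplay ability that posts a character's chat message.
; It activates from a gameplay event, commits its cost, then casts the event's optional object to a chat message wrapper and hands that message to the TextCommunicationSubsystem.
; It ends only on success; a failed cost commit or cast just prints a debug string.
; Both the can-activate and event-response checks always return true.
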(event `self.K2_ActivateAbilityFromEvent`
  (params (EventData :type "GameplayEventData Structure (by ref)"))
  (bind _returnvalue (`self.K2_CommitAbilityCost` false))
  (if _returnvalue
    (bind _ascharacter_chat_message_wrapper (cast `CharacterChatMessageWrapper` (`.OptionalObject` (break `GameplayEventData` EventData)))
      (:`then`
        (`TextCommunicationSubsystem.AddCharacterChatMessage` (subsystem `TextCommunicationSubsystem`) (`CharacterChatMessageWrapper.CharacterChatMessage` _ascharacter_chat_message_wrapper))
        (`self.K2_EndAbility`))
      (:`CastFailed`
        (`KismetSystemLibrary.PrintString` "Can't cast chat message wrapper" true true (struct :`G` 0.66 :`B` 1.0 :`A` 1.0) 5.0)))
    (else
      (`KismetSystemLibrary.PrintString` "Couldn't pass LAST commit Speech Ability Cost" true true (struct :`R` 1.0 :`G` 0.17511 :`B` 0.145262 :`A` 1.0) 5.0))))

(fn `K2_CanActivateAbility`
  (params (ActorInfo :type "GameplayAbilityActorInfo Structure") (Handle :type "GameplayAbilitySpecHandle Structure"))
  (returns (RelevantTags :type "GameplayTagContainer Structure") (ReturnValue :type Boolean))
  (return (struct) true))

(fn `K2_ShouldAbilityRespondToEvent`
  (params (ActorInfo :type "GameplayAbilityActorInfo Structure") (Payload :type "GameplayEventData Structure"))
  (returns (ReturnValue :type Boolean))
  (return true))