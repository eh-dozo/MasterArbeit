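; Gameplay ability for the turn-based combat system that fully restores its owner.
; On activation it applies GE_Heal to itself, with a set-by-caller heal magnitude equal to MaxHealth minus current Health from CombatAttributeSet.
; It then applies GE_RestoreTurnPoints to itself and ends immediately.
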(event `self.K2_ActivateAbility`
  (bind _returnvalue (`self.GetAbilitySystemComponentFromActorInfo`))
  (bind _returnvalue_2 (`AbilitySystemComponent.GetAttributeSet` (`self.GetAbilitySystemComponentFromActorInfo`) "/Script/TurnBasedCombatSystem.CombatAttributeSet"))
  (bind _returnvalue_3 (`AbilitySystemBlueprintLibrary.MakeSpecHandleByClass` "/Game/LongLiveMadness/TurnBasedSystem/GameplayEffect/GE_Heal.GE_Heal_C"))
  (bind _returnvalue_4 (`AbilitySystemBlueprintLibrary.AssignTagSetByCallerMagnitude` _returnvalue_3 (struct :`TagName` "Abilities.Parameters.Heal") (- (`.CurrentValue` (break `GameplayAttributeData` (`CombatAttributeSet.MaxHealth` _returnvalue_2))) (`.CurrentValue` (break `GameplayAttributeData` (`CombatAttributeSet.Health` _returnvalue_2))))))
  (`AbilitySystemComponent.BP_ApplyGameplayEffectSpecToSelf` _returnvalue _returnvalue_4)
  (`AbilitySystemComponent.BP_ApplyGameplayEffectToSelf` :`self` _returnvalue :`GameplayEffectClass` "/Game/LongLiveMadness/TurnBasedSystem/GameplayEffect/GE_RestoreTurnPoints.GE_RestoreTurnPoints_C")
  (`self.K2_EndAbility`))