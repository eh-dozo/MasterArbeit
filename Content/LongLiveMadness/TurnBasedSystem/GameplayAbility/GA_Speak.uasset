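; GA_Speak is an event-triggered gameplay ability that lets a character speak by posting a chat message.
; It unwraps the message from the event's CharacterChatMessageWrapper payload, adds it to the TextCommunicationSubsystem, then ends.
; Activation requires the parent check to pass and an ability system attribute to be at least Cost.
; The cost commit on ability end sits behind an always-false branch, so it never runs.
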(event `self.K2_ActivateAbilityFromEvent`
  (params (EventData :type "GameplayEventData Structure (by ref)"))
  (bind _ascharacter_chat_message_wrapper (cast `CharacterChatMessageWrapper` (`.OptionalObject` (break `GameplayEventData` EventData)))
    (:`then`
      (`TextCommunicationSubsystem.AddCharacterChatMessage` (subsystem `TextCommunicationSubsystem`) (`CharacterChatMessageWrapper.CharacterChatMessage` _ascharacter_chat_message_wrapper))
      (`self.K2_EndAbility`))
    (:`CastFailed`
      (`KismetSystemLibrary.PrintString` "Can't cast chat message wrapper" true true (struct :`G` 0.66 :`B` 1.0 :`A` 1.0) 5.0))))

(event `self.K2_OnEndAbility`
  (params (bWasCancelled :type Boolean))
  (if (not true)
    (bind _returnvalue (`self.K2_CommitAbilityCost` false))
    (if _returnvalue
      (`KismetSystemLibrary.PrintString` "yes")
      (else
        (`KismetSystemLibrary.PrintString` "No")))))

(fn `K2_CanActivateAbility`
  (params (ActorInfo :type "GameplayAbilityActorInfo Structure") (Handle :type "GameplayAbilitySpecHandle Structure"))
  (returns (RelevantTags :type "GameplayTagContainer Structure") (ReturnValue :type Boolean))
  (bind (_bsuccessfullyfoundattribute _returnvalue) (`AbilitySystemBlueprintLibrary.GetFloatAttributeFromAbilitySystemComponent` (`.AbilitySystemComponent` (break `GameplayAbilityActorInfo` ActorInfo)) (struct :`AttributeName` "ActionPoints" :`Attribute` "/Script/TurnBasedCombatSystem.CombatAttributeSet:ActionPoints" :`AttributeOwner` "/Script/CoreUObject.Class'/Script/TurnBasedCombatSystem.CombatAttributeSet'")))
  (bind (_relevanttags _returnvalue_2) (`parent.K2_CanActivateAbility` ActorInfo Handle))
  (if _returnvalue_2
    (if _bsuccessfullyfoundattribute
      (return (struct) (>= _returnvalue (`self.Cost`)))
      (else
        _)))
  (return (struct) false))