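; BP_STT_Move is a StateTree task that moves a Llama agent through a turn-cost gameplay ability.
; On entering the state it wraps distance and a player-character target, a temporary choice, into a movement action sent as a gameplay event payload.
; Seek, Flee and Orbit all trigger the Seek event, while other primitives have no tag.
; The task finishes when the Seek ability's end delegate fires, relying on per-actor-style instancing.
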(event `self.ReceiveLatentEnterState`
  (params (Transition :type "StateTreeTransitionResult Structure (by ref)"))
  (bind _character (`self.Character`))
  (bind _movementdistance (`self.MovementDistance`))
  (bind _returnvalue (select `EMovementPrimitive` (`self.MovementPrimitive`) :`Seek` (struct :`TagName` "Abilities.Event.Llama.Seek") :`Flee` (struct :`TagName` "Abilities.Event.Llama.Seek") :`Orbit` (struct :`TagName` "Abilities.Event.Llama.Seek") :!type "GameplayTag Structure"))
  (bind _asturn_cost_gameplay_ability (cast `TurnCostGameplayAbility` (`.ReturnValue` (`AbilitySystemBlueprintLibrary.GetGameplayAbilityFromSpecHandle` (`MasterArbeitCharacter.AbilitySystemComponent` _character) (`/Game/LongLiveMadness/LlamaAgent/BP_BaseAgentCharacter.Seek_SH` _character))))
    (:`then`
      (bind _output_get (set `self.MovementAbility` _asturn_cost_gameplay_ability))
      (add `TurnCostGameplayAbility.OnAbilityEnded` _output_get (delegate `OnMovementAbilityEnd`)) ; THIS ONLY WORKS BECAUSE THE GAS ABILITY HAS ITS "Instancing Policy" SET TO "Per Player"\n-> i.e. it keep the state and binds the delegate to the right ability instance
      (bind _returnvalue_2 (`GameplayStatics.GetActorOfClass` "/Game/LongLiveMadness/Player/BP_PlayerCharacter.BP_PlayerCharacter_C")) ; TEMPORARY - REPLACE WITH AUTO-MATCHING FUNCTION
      (bind _returnvalue_3 (`MovementActionWrapper.CreateWrapper` self (make `MovementAction` (`|GetEnumeratorNameAsString` _movementdistance) (select `EMovementDistance` _movementdistance :`Adjacent` 150.0 :`Near` 300.0 :`Moderate` 600.0 :`Far` 900.0 :!type "Float (single-precision)") _returnvalue_2)))
      (`AbilitySystemBlueprintLibrary.SendGameplayEventToActor` (`self.Character`) _returnvalue (make `GameplayEventData` _returnvalue null null _returnvalue_3)))
    (:`CastFailed`
      (`KismetSystemLibrary.PrintString` "STT Move: Can't cast movement ability" true true (struct :`R` 1.0 :`G` 0.054122 :`A` 1.0) 20.0))))

(event `OnMovementAbilityEnd`
  (clear `TurnCostGameplayAbility.OnAbilityEnded` (`self.MovementAbility`))
  (`self.FinishTask` true))