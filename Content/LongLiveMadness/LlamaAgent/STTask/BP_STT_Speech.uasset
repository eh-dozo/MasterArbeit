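; BP_STT_Speech is a StateTree task that makes an LLM-driven character speak in the game.
; On state entry it wraps a chat message, built from the character's group name, theme color and either the content, an ellipsis for silence or an invalid placeholder, in a CharacterChatMessageWrapper.
; It sends that wrapper to the character as the optional object of an Abilities.Event.Speech gameplay event, then immediately finishes successfully.
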(event `self.ReceiveLatentEnterState`
  (params (Transition :type "StateTreeTransitionResult Structure (by ref)"))
  (bind _character (`self.Character`))
  (bind _character_2 (`self.Character`))
  (bind _returnvalue (`|GenericCreateObject` "/Script/MasterArbeit.CharacterChatMessageWrapper" (make `CharacterChatMessage` (`MasterArbeitCharacter.CharacterGroupName` _character) (select `EVerbalResponseType` (`self.Type`) :`Speech` (`KismetTextLibrary.Conv_StringToText` (`self.Content`)) :`Silence` "..." :`Invalid` "INVALID") (`/Game/LongLiveMadness/Core/BP_BaseCharacter.ThemeColor` _character))))
  (`AbilitySystemBlueprintLibrary.SendGameplayEventToActor` _character_2 (struct :`TagName` "Abilities.Event.Speech") (make `GameplayEventData` (struct :`TagName` "Abilities.Event.Speech") _character_2 _character_2 _returnvalue))
  (`self.FinishTask` true))