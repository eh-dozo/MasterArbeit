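; StateTree task that primes a llama.cpp-driven character with a system prompt and chat history so it can reason.
; On state entry it gathers the rows of a chat history DataTable into an array, then pops the last message.
; It passes the system prompt, remaining history as few-shot examples and popped message as initial user prompt to SwitchCharacter.
; It then sets HasTought and finishes successfully without waiting for a reply.
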(event `self.ReceiveLatentEnterState`
  (params (Transition :type "StateTreeTransitionResult Structure (by ref)"))
  (bind _chathistorydatatable (`self.ChatHistoryDataTable`))
  (bind _chathistory (`self.ChatHistory`))
  (bind _returnvalue (`KismetArrayLibrary.Array_LastIndex` _chathistory))
  (bind _outrownames (`DataTableFunctionLibrary.GetDataTableRowNames` _chathistorydatatable))
  (for _array_element _outrownames
    (bind _returnvalue_2 (`|GetDataTableRow` _chathistorydatatable _array_element)
      (:`then`
        (`KismetArrayLibrary.Array_AddUnique` (`self.ChatHistory`) _returnvalue_2))))
  (bind _output_get (set `self.LastChat` (`|GetArrayItem` _chathistory _returnvalue)))
  (`KismetArrayLibrary.Array_Remove` _chathistory _returnvalue)
  (`LlamaCppSubsystem.SwitchCharacter` (subsystem `LlamaCppSubsystem`) (`KismetTextLibrary.Conv_TextToString` (`SystemPromptDataAsset.SystemPrompt` (`self.SystemPrompt`))) _chathistory (`.Content` (break `ChatMessage` _output_get)))
  (set `self.HasTought` true)
  (`self.FinishTask` true))