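; Base Blueprint for a Llama agent character, a turn-based unit that receives its movement abilities through the Gameplay Ability System.
; On StartUnitTurn it runs the parent logic, then grants the Seek, Flee and Orbit movement abilities and stores each spec handle.
; It then calls OnTurnStart.
; The grants repeat on every StartUnitTurn call, and this Blueprint neither activates nor removes them.
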(event `self.StartUnitTurn`
  (`parent.StartUnitTurn`)
  (bind _returnvalue (`AbilitySystemComponent.K2_GiveAbility` (`self.AbilitySystemComponent`) "/Game/LongLiveMadness/LlamaAgent/GAbilities/GA_LlamaMovement_Seek.GA_LlamaMovement_Seek_C" 0 -1))
  (set `self.Seek_SH` _returnvalue)
  (bind _returnvalue_2 (`AbilitySystemComponent.K2_GiveAbility` (`self.AbilitySystemComponent`) "/Game/LongLiveMadness/LlamaAgent/GAbilities/GA_LlamaMovement_Flee.GA_LlamaMovement_Flee_C" 0 -1))
  (set `self.Flee_SH` _returnvalue_2)
  (bind _returnvalue_3 (`AbilitySystemComponent.K2_GiveAbility` (`self.AbilitySystemComponent`) "/Game/LongLiveMadness/LlamaAgent/GAbilities/GA_LlamaMovement_Orbit.GA_LlamaMovement_Orbit_C" 0 -1))
  (set `self.Orbit_SH` _returnvalue_3)
  (`self.OnTurnStart`))

(fn `UserConstructionScript`
  (`parent.UserConstructionScript`))