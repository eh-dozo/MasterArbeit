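; GA_LlamaMovement_Seek is a gameplay ability that moves an AI agent to a set distance from a target character.
; It reads the movement action from the event payload and snaps the destination to a grid tile center, on the line from target toward agent.
; It cancels if the agent is already near that tile or movement fails.
; On arrival, it records the move, with the target's name, in the agent's TurnActionTracker.
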(event `self.K2_ActivateAbilityFromEvent`
  (params (EventData :type "GameplayEventData Structure (by ref)"))
  (bind _returnvalue (`self.GetOwningActorFromActorInfo`))
  (`parent.K2_ActivateAbilityFromEvent` EventData)
  (bind _asmovement_action_wrapper (cast `MovementActionWrapper` (`.OptionalObject` (break `GameplayEventData` EventData)))
    (:`then`
      (bind _gridactor (message `/Game/LongLiveMadness/Core/BPI_InGameGM.GetGridActor` (`GameplayStatics.GetGameMode`)))
      (bind (_distanceliteral _distance _target) (break `MovementAction` (`MovementActionWrapper.MovementAction` _asmovement_action_wrapper)))
      (bind _returnvalue_2 (`Actor.K2_GetActorLocation` _target))
      (bind _outtilecenter (`LandscapeGrid.LocateTileCenter` _gridactor (+ (* _distance (`KismetMathLibrary.Normal` (- (`Actor.K2_GetActorLocation` (`self.GetOwningActorFromActorInfo`)) _returnvalue_2))) _returnvalue_2)))
      (bind _outtilecenter_2 (`LandscapeGrid.LocateTileCenter` _gridactor (`Actor.K2_GetActorLocation` _returnvalue)))
      (if (== _outtilecenter_2 _outtilecenter :`ErrorTolerance` 50.0)
        (`KismetSystemLibrary.PrintString` "Cancel Agent Seek Ability: AI Already at target loc" false)
        (`self.K2_CancelAbility`)
        (else
          (bind _asbp_base_agent_character (cast `/Game/LongLiveMadness/LlamaAgent/BP_BaseAgentCharacter` _returnvalue))
          (`GATSimpleCharacterMoveTo.WaitForCharacterMovementToComplete` _outtilecenter
            (:`then`
              (`KismetSystemLibrary.PrintString` "Starting task" false))
            (:`OnMovementComplete`
              (bind _asbp_base_character (cast `/Game/LongLiveMadness/Core/BP_BaseCharacter` _target)
                (:`then`
                  (`TurnActionTrackerComponent.RecordMovement` (`/Game/LongLiveMadness/Core/BP_BaseCharacter.TurnActionTracker` _asbp_base_agent_character) (`KismetTextLibrary.Conv_TextToString` (`|FormatText` "moved \"{0}\" toward {1}" _distanceliteral (select `ECharacterGroupName` (`MasterArbeitCharacter.CharacterGroupName` _asbp_base_character) :`Default` "Invalid" :`Player` "Mercenary" :`Green` "Aldric" :`Red` "Grimnar" :`Purple` "Lucien"))))
                  (`self.K2_EndAbility`))
                (:`CastFailed`
                  (`KismetSystemLibrary.PrintString` "Cancel Llama Seek: can't cast character" false true (struct :`R` 1.0 :`G` 0.059236 :`A` 1.0) 20.0)
                  (`self.K2_CancelAbility`))))
            (:`OnMovementFailed`
              (`KismetSystemLibrary.PrintString` "Cancel Agent Seek Ability: Fail AI Move To" false)
              (`self.K2_CancelAbility`))))))
    (:`CastFailed`
      (`KismetSystemLibrary.PrintString` "Cancel Llama Seek: can't cast wrapper" false true (struct :`R` 1.0 :`G` 0.059236 :`A` 1.0) 20.0)
      (`self.K2_CancelAbility`))))